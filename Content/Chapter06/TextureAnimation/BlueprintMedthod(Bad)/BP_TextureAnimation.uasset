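; Actor Blueprint that plays a flipbook-style texture animation on its Plane by swapping textures from Blueprint.
; A looping timer started on BeginPlay fires at about 30 frames per second, advancing an index that wraps at a hardcoded frame count.
; Each step calls CreateDynamicMaterialInstance again rather than using a stored instance, then sets the CurrentFrame texture parameter from TextureArray.
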(event Custom|NextFrame
  (bind _returnvalue (Rendering|Material|CreateDynamicMaterialInstance (Variables|Default|GetPlane) 0 "/Game/Chapter06/TextureAnimation/BlueprintMedthod(Bad)/M_TextureAnimationBlueprint.M_TextureAnimationBlueprint" "None" :!class /Script/Engine.PrimitiveComponent))
  (bind _output_get (Variables|Default|SetIndex (Math|Integer|%(Integer) (+ (Variables|Default|GetIndex) 1) 2)))
  (Rendering|Material|SetTextureParameterValue _returnvalue "CurrentFrame" (Utilities|Array|Get(acopy) (Variables|Default|GetTextureArray) _output_get)))

(event EventBeginPlay
  ;[0.15 0.15 0.15 0.5] Time = 1 / framrate
  (Utilities|Time|SetTimerbyEvent (delegate Custom|NextFrame) 0.03333 true))

(event Collision|EventActorBeginOverlap
  (params (OtherActor :type Actor%20Object%20Reference)))

(event EventTick
  (params (DeltaSeconds :type Float%20%28single-precision%29)))

(fn ConstructionScript)